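; BP_PlayerWall is a wall actor that shows its remaining health through its color.
; On BeginPlay it creates a dynamic material instance from the Cube's first material and assigns it back to the mesh.
; When damage is received, it sets the material's Color parameter by blending from red to green according to the ratio of Health to MaxHealth.
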(event `self.ReceiveBeginPlay`
  (bind _returnvalue (`KismetMaterialLibrary.CreateDynamicMaterialInstance` (`PrimitiveComponent.GetMaterial` (`self.Cube`) 0) "None" "Transient"))
  (bind _output_get (set `self.MaterialInstance` _returnvalue))
  (`PrimitiveComponent.SetMaterial` (`self.Cube`) 0 _output_get))

(event `self.OnDamageReceived`
  (params (PreviousHealth :type Integer))
  (`MaterialInstanceDynamic.SetVectorParameterValue` (`self.MaterialInstance`) "Color" (`KismetMathLibrary.LinearColorLerp` (struct :`R` 1.0 :`G` 0.056849 :`A` 1.0) (struct :`R` 0.004252 :`G` 1.0 :`A` 1.0) (/ (`self.Health`) (`self.MaxHealth`)))))

(fn `UserConstructionScript`)